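; BP_TempController is a temporary player controller that brings up the main menu, settings and input at startup.
; On BeginPlay it creates the main widget container, opens WBP_MainMenu in it and sets UI-only input focused on that menu.
; It then reads and loads saved settings through the settings subsystem and adds a rebind-test Enhanced Input mapping context.
; A debug T key prints the last confirmed screen resolution.
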(event EventBeginPlay
  (bind _returnvalue (Subsystems|GetSettingsSubsystem))
  (bind _self self)
  (bind _returnvalue_2 (PlayerController|LocalPlayerSubsystems|GetEnhancedInputLocalPlayerSubsystem _self))
  (Utilities|FlowControl|Sequence
    (:then_0
      (bind _returnvalue_3 (UserInterface|CreateWidget "/SimpleSettings/Widget/WBP_MainWidgetContainer.WBP_MainWidgetContainer_C"))
      (bind _output_get (Variables|Default|SetMainContainer _returnvalue_3))
      (UserInterface|Viewport|AddtoViewport _output_get 0)
      (bind _returnvalue_4 (Default|OpenWidget (Variables|Default|GetMainContainer) "/SimpleSettings/Widget/WBP_MainMenu.WBP_MainMenu_C"))
      (Input|SetInputModeUIOnly self _returnvalue_4 "DoNotLock" false))
    (:then_1
      (Variables|/Script/SimpleSettings.SettingsSubsystem|SetSettingsSaveData _returnvalue "/SimpleSettings/Blueprints/SG_SettingsData.SG_SettingsData_C")
      (Class|SettingsSubsystem|ReadSettingsData _returnvalue)
      (Class|SettingsSubsystem|LoadSettingsData _returnvalue (Variables|/Script/SimpleSettings.SettingsSubsystem|GetPlayerDisplaySettings _returnvalue)))
    (:then_2
      (Utilities|IsValid _returnvalue_2
        (:Is%20Valid
          (Input|AddMappingContext _returnvalue_2 "/SimpleSettings/Input/IMC_TestReBind.IMC_TestReBind" 0 "(bIgnoreAllPressedKeysUntilRelease=True,bForceImmediately=False)"))))))

(event Input|KeyboardEvents|DebugKeyT
  (params (Key :type Key%20Structure :default "None") (ActionValue :type Input%20Action%20Value%20Structure))
  (:Pressed
    (bind _returnvalue (Settings|GetGameUserSettings))
    (Development|PrintString (Utilities|String|ToString(Integer) (Class|GameUserSettings|GetLastConfirmedScreenResolution _returnvalue)))))

(fn ConstructionScript)